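; BP_NoC_Character is a player-controlled character that moves on two input axes and turns its mesh to face the input direction.
; MoveForward and MoveRight apply movement along the actor's forward and right vectors and store their axis values in a Movement vector.
; While that vector is non-zero, Tick sets the mesh's relative yaw with atan2, rotating only the mesh and leaving the actor's movement axes unchanged.
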(event `self.ReceiveTick`
  (params (DeltaSeconds :type "Float (single-precision)"))
  (bind (_movement_x _movement_y) (`KismetMathLibrary.BreakVector` (`self.Movement`)))
  (if (> (`KismetMathLibrary.VSize` (`self.Movement`)) 0.0)
    (`SceneComponent.K2_SetRelativeRotation` (`self.Mesh`) (`KismetMathLibrary.MakeRotator` 0.0 0.0 (`KismetMathLibrary.DegAtan2` (* _movement_y -1.0) _movement_x)) false false)))

(event `InputAxis|MoveForward`
  (params (AxisValue :type "Float (single-precision)"))
  (bind (_movement_x _movement_y _movement_z) (`KismetMathLibrary.BreakVector` (`self.Movement`)))
  (set `self.Movement` (`KismetMathLibrary.MakeVector` _movement_x AxisValue _movement_z))
  (`self.AddMovementInput` (`self.GetActorForwardVector`) AxisValue))

(event `InputAxis|MoveRight`
  (params (AxisValue :type "Float (single-precision)"))
  (bind (_movement_x _movement_y _movement_z) (`KismetMathLibrary.BreakVector` (`self.Movement`)))
  (set `self.Movement` (`KismetMathLibrary.MakeVector` AxisValue _movement_y _movement_z))
  (`self.AddMovementInput` (`self.GetActorRightVector`) AxisValue))

(fn `UserConstructionScript`)